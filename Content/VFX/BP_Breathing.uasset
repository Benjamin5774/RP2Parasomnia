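; BP_Breathing is a Blueprint that drives a smoothed breathing visual effect through material parameters.
; Each tick it sets breathing and FOV targets from the IsBreathing flag, slightly narrowing the FOV value while breathing.
; It eases both values with FInterpTo and writes them to the MPC_Focus and MPC_Breathing parameter collections, for materials such as post-process to read.
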(event `self.ReceiveTick`
  (params (DeltaSeconds :type "Float (single-precision)"))
  (`|ExecutionSequence`
    (:`then_0`
      ; Breathing Effect
      (if (`self.IsBreathing`)
        (set `self.TargetBreathingValue` 1.0)
        (set `self.TargetFOV` 0.9)
        (else
          (set `self.TargetBreathingValue` 0.0)
          (set `self.TargetFOV` 1.0))))
    (:`then_1`
      (`|ExecutionSequence`
        (:`then_0`
          ;; FOV
          (bind _output_get (set `self.FOV` (`KismetMathLibrary.FInterpTo` (`self.FOV`) (`self.TargetFOV`) DeltaSeconds 2.0)))
          (`KismetMaterialLibrary.SetScalarParameterValue` "/Game/VFX/MPC_Focus.MPC_Focus" "FOV" _output_get))
        (:`then_1`
          ;; Post-Process
          (bind _output_get_2 (set `self.BreathingValue` (`KismetMathLibrary.FInterpTo` (`self.BreathingValue`) (`self.TargetBreathingValue`) DeltaSeconds 2.0)))
          (`KismetMaterialLibrary.SetScalarParameterValue` "/Game/VFX/MPC_Breathing.MPC_Breathing" "BreathingValue" _output_get_2))))))