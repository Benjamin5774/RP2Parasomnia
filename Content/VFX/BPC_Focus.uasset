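; BPC_Focus is a component that detects which BP_Animation actor its owning pawn's camera is looking at.
; BeginPlay caches the pawn's camera component.
; Every tick, a long Visibility line trace runs along the camera's forward vector, with one-frame debug drawing, and calls Focused on any BP_Animation it hits.
; An unconnected node targets the MPC_Focus parameter collection but never runs.
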(event `self.ReceiveBeginPlay`
  (bind _aspawn (cast `Pawn` (`self.GetOwner`)))
  (set `self.CameraActor` (`Actor.GetComponentByClass` _aspawn "/Script/Engine.CameraComponent")))

(event `self.ReceiveTick`
  (params (DeltaSeconds :type "Float (single-precision)"))
  (bind _cameraactor (`self.CameraActor`))
  (bind _returnvalue (`SceneComponent.K2_GetComponentLocation` _cameraactor))
  (bind _outhit (`KismetSystemLibrary.LineTraceSingle` :`Start` _returnvalue :`End` (+ _returnvalue (* (`SceneComponent.GetForwardVector` _cameraactor) 10000.0)) :`TraceChannel` "TraceTypeQuery1" :`DrawDebugType` "ForOneFrame"))
  (bind _asbp_animation (cast `/Game/VFX/BluePrint/BP_Animation` (`.HitActor` (`GameplayStatics.BreakHitResult` _outhit))))
  (`/Game/VFX/BluePrint/BP_Animation.Focused` _asbp_animation))