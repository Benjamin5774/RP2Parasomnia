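; Clock actor that blends its animation between normal and surreal states according to how recently it was focused.
; Focused resets a timer; once Tick pushes it past FocusTime, an interpolated value eases toward surreal and feeds ABP_Clock's LerpValue.
; Custom depth stencil marks the clock while the timer is under one second.
; A helper creates dynamic material instances but is not called here.
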(event `self.ReceiveBeginPlay`
  (bind _asabp_clock (cast `/Game/Art/Clock/ABP_Clock` (`SkeletalMeshComponent.GetAnimInstance` (`self.Clock`))))
  (set `self.As ABP Clock` _asabp_clock))

(event `self.ReceiveTick`
  (params (DeltaSeconds :type "Float (single-precision)"))
  (bind _clock (`self.Clock`))
  (bind _clock_2 (`self.Clock`))
  (set `self.Timer` (+ DeltaSeconds (`self.Timer`)))
  (`|ExecutionSequence`
    (:`then_0`
      ; Calculate Animation Lerp Value (0:Normal, 1:Surrealism)
      (if (> (`self.Timer`) (`self.FocusTime`))
        (set `self.TargetValue` 1.0)
        (else
          (set `self.TargetValue` 0.0)))
      (bind _output_get (set `self.LerpValue0` (`KismetMathLibrary.FInterpTo` (`self.LerpValue0`) (`self.TargetValue`) DeltaSeconds 0.5)))
      (set `/Game/Art/Clock/ABP_Clock.LerpValue` _output_get (`self.As ABP Clock`)))
    (:`then_1`
      (if (< (`self.Timer`) 1.0)
        (`PrimitiveComponent.SetRenderCustomDepth` _clock_2 true)
        (`PrimitiveComponent.SetCustomDepthStencilValue` _clock_2 1)
        (else
          (`PrimitiveComponent.SetRenderCustomDepth` _clock true)
          (`PrimitiveComponent.SetCustomDepthStencilValue` _clock 0))))))

(event `Focused`
  (set `self.IsFocused` true)
  (set `self.Timer` 0.0))

(fn `SetupDynaMaterial`
  (params (MeshComponent :type "StaticMeshComponent Object Reference") (Material :type "Material Object Reference"))
  (`PrimitiveComponent.CreateDynamicMaterialInstance` MeshComponent 0 Material "None"))

(fn `UserConstructionScript`)