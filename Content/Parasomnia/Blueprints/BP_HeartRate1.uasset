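; BP_HeartRate1 is a Blueprint that simulates a heart rate value driven by a breathing state.
; Each Tick, it uses FInterpTo to ease HeartRate toward MaxHeartRate while IsBreathing is true, and toward MinHeartRate otherwise, with separate increase and decrease speeds.
; The graph only updates the value; nothing here sets IsBreathing or acts on HeartRate.
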(event `self.ReceiveTick`
  (params (DeltaSeconds :type "Float (single-precision)"))
  (if (`self.bIsBreathing`)
    (set `self.HeartRate` (`KismetMathLibrary.FInterpTo` (`self.HeartRate`) (`self.MaxHeartRate`) DeltaSeconds (`self.IncreaseRate`)))
    (else
      (set `self.HeartRate` (`KismetMathLibrary.FInterpTo` (`self.HeartRate`) (`self.MinHeartRate`) DeltaSeconds (`self.DecreaseRate`))))))

(fn `UserConstructionScript`)