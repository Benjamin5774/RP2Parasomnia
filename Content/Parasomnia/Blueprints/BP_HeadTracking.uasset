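; BP_HeadTracking is an unfinished Blueprint that makes a single view-center line trace at BeginPlay.
; It deprojects the viewport center for the first player controller and traces on the Visibility channel from that point.
; The trace end is the scaled view direction without the start position added, so it is relative to the world origin.
; The hit result is unused, Tick is disabled, and no tracking is implemented.
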(event `self.ReceiveBeginPlay`
  (bind (_x _y) (`KismetMathLibrary.BreakVector2D` (`WidgetLayoutLibrary.GetViewportSize`)))
  (`|ExecutionSequence`
    (:`then_0`
      (bind (_worldposition _worlddirection) (`GameplayStatics.DeprojectScreenToWorld` (`GameplayStatics.GetPlayerController` 0) (`KismetMathLibrary.MakeVector2D` (/ _x 2.0) (/ _y 2.0))))
      (bind (_outhit _returnvalue) (`KismetSystemLibrary.LineTraceSingle` _worldposition (* _worlddirection 5000.0) "TraceTypeQuery1")))))

(fn `UserConstructionScript`)